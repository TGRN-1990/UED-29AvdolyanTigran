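; Arena door that swings open and closed through an OpenDoor event, usable while a BP_Character_Base is in its overlap volume and that character's ItemKeyCount equals three.
; A timeline rotates the mesh up to 90 degrees, choosing the swing side by dot product with the player's position, and reverses to close.
; A sound spawns on every timeline update.
; With any other key count, OpenDoor sets ItemKeyCount to 4.
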(event OnComponentBeginOverlap(PlayerColl)
  (params (OverlappedComponent :type Primitive%20Component%20Object%20Reference) (OtherActor :type Actor%20Object%20Reference) (OtherComp :type Primitive%20Component%20Object%20Reference) (OtherBodyIndex :type Integer) (bFromSweep :type Boolean) (SweepResult :type Hit%20Result%20Structure%20%28by%20ref%29))
  (bind _asbp_character_base (Utilities|Casting|CastToBP_Character_Base OtherActor))
  (Variables|Default|SetPlayerRef _asbp_character_base)
  (Variables|Default|SetBlock%20Logik false))

(event OnComponentEndOverlap(PlayerColl)
  (params (OverlappedComponent :type Primitive%20Component%20Object%20Reference) (OtherActor :type Actor%20Object%20Reference) (OtherComp :type Primitive%20Component%20Object%20Reference) (OtherBodyIndex :type Integer))
  (Utilities|Casting|CastToBP_Character_Base OtherActor)
  (Variables|Default|SetBlock%20Logik true))

(event Custom|OpenDoor
  (bind _defaultsceneroot (Variables|Actor|GetDefaultSceneRoot))
  (if (not (Variables|Default|GetBlock%20Logik))
    (bind _asbp_character_base (Utilities|Casting|CastToBP_Character_Base (Variables|Default|GetPlayerRef)))
    (if (== (Variables|/Game/Blueprints/Base/BP_Character_Base.BP_Character_Base_C|GetItemKeyCount _asbp_character_base) 3)
      (if (Variables|Default|GetIsDoorClosed)
        (Variables|Default|SetIsDoorClosed false)
        (Variables|Default|SetDotProduct (Math|Vector|DotProduct (Math|Vector|Normalize (- (Transformation|GetWorldLocation _defaultsceneroot) (Transformation|GetActorLocation (Variables|Default|GetPlayerRef)))) (Math|Vector|GetForwardVector _defaultsceneroot)))
        (bind (_direction _newtrack_0) (Timeline|Timeline_0 Play)
          (:Update
            (Transformation|SetRelativeRotation (Variables|Default|GetStaticMesh) (Math|Rotator|MakeRotator 0.0 0.0 (Math|Float|Lerp 0.0 (Math|Float|SelectFloat -9e+01 9e+01 (>= (Variables|Default|GetDotProduct) 0.0)) _newtrack_0)) false false)
            (Audio|SpawnSound2D "/Game/Retro_8Bit_Sounds/Jumping/Cues/retro_jump_bounce_09_Cue.retro_jump_bounce_09_Cue" 1.0 1.0 0.0 0))
          (:Finished
            (switch Utilities|FlowControl|Switch|SwitchonETimelineDirection _direction
              (:Backward
                (Variables|Default|SetIsDoorClosed true)))))
        (else
          (Timeline|Timeline_0 Reverse)))
      (else
        (bind _asbp_character_base_2 (Utilities|Casting|CastToBP_Character_Base (Variables|Default|GetPlayerRef)))
        (Variables|/Game/Blueprints/Base/BP_Character_Base.BP_Character_Base_C|SetItemKeyCount _asbp_character_base_2 4)))))

(fn ConstructionScript)