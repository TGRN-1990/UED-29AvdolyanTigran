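; DoorKey is an arena pickup that gives a character a key.
; A box overlap stores the overlapping BP_Character_Base and toggles a lootable flag on enter and exit.
; The Looting event, if the flag is set, increments that character's key count, sets its BPKeyUp flag, prints the count, plays a 2D sound and destroys the actor.
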(event OnComponentBeginOverlap(Box)
  (params (OverlappedComponent :type Primitive%20Component%20Object%20Reference) (OtherActor :type Actor%20Object%20Reference) (OtherComp :type Primitive%20Component%20Object%20Reference) (OtherBodyIndex :type Integer) (bFromSweep :type Boolean) (SweepResult :type Hit%20Result%20Structure%20%28by%20ref%29))
  (bind _asbp_character_base (Utilities|Casting|CastToBP_Character_Base OtherActor))
  (Variables|Default|SetRefColl _asbp_character_base)
  (Variables|Default|SetItem_loot true))

(event OnComponentEndOverlap(Box)
  (params (OverlappedComponent :type Primitive%20Component%20Object%20Reference) (OtherActor :type Actor%20Object%20Reference) (OtherComp :type Primitive%20Component%20Object%20Reference) (OtherBodyIndex :type Integer))
  (Utilities|Casting|CastToBP_Character_Base OtherActor)
  (Variables|Default|SetItem_loot false))

(event Custom|Looting
  (if (Variables|Default|GetItem_loot)
    (bind _asbp_character_base (Utilities|Casting|CastToBP_Character_Base (Variables|Default|GetRefColl)))
    (bind _output_get (Variables|/Game/Blueprints/Base/BP_Character_Base.BP_Character_Base_C|SetItemKeyCount _asbp_character_base (+ (Variables|/Game/Blueprints/Base/BP_Character_Base.BP_Character_Base_C|GetItemKeyCount _asbp_character_base) 1)))
    (Development|PrintString (Utilities|String|ToString(Byte) _output_get) true true "(R=0.401042,G=0.534674,B=1.000000,A=1.000000)" 3.0)
    (Variables|/Game/Blueprints/Base/BP_Character_Base.BP_Character_Base_C|SetBP_KeyUp _asbp_character_base true)
    (Audio|SpawnSound2D "/Game/Retro_8Bit_Sounds/Jumping/Cues/retro_jump_bounce_13_Cue.retro_jump_bounce_13_Cue" 1.0 1.0 0.0 0)
    (Actor|DestroyActor self)))

(fn ConstructionScript)