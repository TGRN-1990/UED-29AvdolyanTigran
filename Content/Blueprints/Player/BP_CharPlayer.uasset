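; BP_CharPlayer is the player character Blueprint, handling AI noise, stat updates and death.
; It reports a noise event at the capsule every second, with loudness lowered while the BP_CharControlls controller has Crouch set.
; BPCharStats status updates either refresh the lifebar and hand the character to its BP_widjet_bar widget, or trigger death.
; Death plays a 2D alarm siren, then destroys the actor after a short delay.
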(event Custom|DeadHero
  (Audio|SpawnSound2D "/Game/Retro_8Bit_Sounds/Alarms_Sirens/Wavs/retro_alarm_siren_loop_12.retro_alarm_siren_loop_12" 1.0 1.0 0.0 0)
  (Utilities|FlowControl|Delay 1.0)
  (Actor|DestroyActor))

(event EventBeginPlay
  (bind _bp_char_stats (Variables|Default|GetBP_Char_Stats))
  (|CallParentFunction)
  (Utilities|FlowControl|Sequence
    (:then_0
      (Utilities|FlowControl|Delay 1.0 :!label _label)
      (Class|AISenseHearing|ReportNoiseEvent (Transformation|GetWorldLocation (Variables|Default|GetCapsuleComponent)) (Variables|Default|GetLoudness_1or3/4) self 0.0 "None")
      (goto _label))
    (:then_1
      (EventDispatchers|BindEventtoOnStatusUpdate (Variables|Default|GetBP_Char_Stats) (EventDispatchers|CreateEvent :!event BPPlayerStatUpdated))
      (CallFunction|PlayerStatUpdated self false false (Variables|/Game/Blueprints/Companent/BP_Char_Stats.BP_Char_Stats_C|GetCurrentHP _bp_char_stats) (Variables|/Game/Blueprints/Companent/BP_Char_Stats.BP_Char_Stats_C|GetCurrentEP _bp_char_stats)))))

(event EventTick
  (params (DeltaSeconds :type Float%20%28single-precision%29))
  (bind _asbp_char_controlls (Utilities|Casting|CastToBP_CharControlls (Game|GetInstigatorController)))
  (if (Variables|/Game/Blueprints/Base/BP_CharControlls.BP_CharControlls_C|GetCrouch+ _asbp_char_controlls)
    (Variables|Default|SetLoudness_1or3/4 0.75)
    (else
      (Variables|Default|SetLoudness_1or3/4 1.0))))

(fn ConstructionScript
  (|CallParentFunction))

(fn BPPlayerStatUpdated
  (params (IsDead :type Boolean) (ItsDamage :type Boolean) (CurrentHP :type Integer) (CurrentEP :type Integer))
  (if IsDead
    (CallFunction|DeadHero)
    (else
      (Default|ConfigLifebar (Variables|Default|GetBP_Char_Stats))
      (bind _asbp_widjet_bar (Utilities|Casting|CastToBP_widjet_bar (UserInterface|GetUserWidgetObject (Variables|Default|GetWidgetChar))))
      (Variables|/Game/Blueprints/BP_HUD/BP_Widjet/BP_widjet_bar.BP_widjet_bar_C|SetBP_charHealht _asbp_widjet_bar self))))