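; BP_Character_Base is a base character Blueprint that delegates lifebar and movement setup to its BPCharStats member on BeginPlay, printing the lifebar setup result on screen.
; Every Tick it casts the instigator controller to BP_CharControlls and copies its Jump and Crouch values into CharJump and CharCrouch.
; Capsule overlaps with a DoorKey store that actor in NearItems, with no clearing on overlap end.
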(event OnComponentBeginOverlap(Capsule)
  (params (OverlappedComponent :type Primitive%20Component%20Object%20Reference) (OtherActor :type Actor%20Object%20Reference) (OtherComp :type Primitive%20Component%20Object%20Reference) (OtherBodyIndex :type Integer) (bFromSweep :type Boolean) (SweepResult :type Hit%20Result%20Structure%20%28by%20ref%29))
  (bind _asdoor_key (Utilities|Casting|CastToDoorKey OtherActor))
  (Variables|Default|SetNear_Items _asdoor_key))

(event EventBeginPlay
  (Utilities|FlowControl|Sequence
    (:then_0
      (bind _lifebare (Default|ConfigLifebar (Variables|Default|GetBP_Char_Stats)))
      (Development|PrintString _lifebare true true "(R=0.000000,G=0.660000,B=1.000000,A=1.000000)" 6e+01))
    (:then_1
      (Default|ConfigMove (Variables|Default|GetBP_Char_Stats)))))

(event EventTick
  (params (DeltaSeconds :type Float%20%28single-precision%29))
  (bind _asbp_char_controlls (Utilities|Casting|CastToBP_CharControlls (Game|GetInstigatorController)))
  (Variables|Default|SetCharJump (Variables|/Game/Blueprints/Base/BP_CharControlls.BP_CharControlls_C|GetJump+ _asbp_char_controlls))
  (Variables|Default|SetCharCrouch (Variables|/Game/Blueprints/Base/BP_CharControlls.BP_CharControlls_C|GetCrouch+ _asbp_char_controlls)))

(fn ConstructionScript)