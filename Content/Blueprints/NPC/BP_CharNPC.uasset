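; NPC character Blueprint that handles its health bar display and death.
; On BeginPlay it binds to the status updates of its BPCharStats component and runs an initial stat update with current HP and EP.
; While alive, a stat update configures the lifebar and passes the NPC to its health widget.
; On death it plays a 2D siren sound and destroys itself after a short delay.
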(event Custom|DeadNPC
  (Audio|SpawnSound2D "/Game/Retro_8Bit_Sounds/Alarms_Sirens/Wavs/retro_alarm_siren_loop_12.retro_alarm_siren_loop_12" 1.0 1.0 0.0 0)
  (Utilities|FlowControl|Delay 1.0)
  (Actor|DestroyActor))

(event EventBeginPlay
  (bind _bp_char_stats (Variables|Default|GetBP_Char_Stats))
  (|CallParentFunction)
  (EventDispatchers|BindEventtoOnStatusUpdate (Variables|Default|GetBP_Char_Stats) (EventDispatchers|CreateEvent :!event BPNPCStatUpdated))
  (CallFunction|NPCStatUpdated self false false (Variables|/Game/Blueprints/Companent/BP_Char_Stats.BP_Char_Stats_C|GetCurrentHP _bp_char_stats) (Variables|/Game/Blueprints/Companent/BP_Char_Stats.BP_Char_Stats_C|GetCurrentEP _bp_char_stats)))

(event Collision|EventActorBeginOverlap
  (params (OtherActor :type Actor%20Object%20Reference))
  (|CallParentFunction OtherActor) ; This node is disabled and will not be called.\nDrag off pins to build functionality.
)

(event EventTick
  (params (DeltaSeconds :type Float%20%28single-precision%29))
  (|CallParentFunction DeltaSeconds) ; This node is disabled and will not be called.\nDrag off pins to build functionality.
)

(fn ConstructionScript
  (|CallParentFunction))

(fn BPNPCStatUpdated
  (params (IsDead :type Boolean) (ItsDamage :type Boolean) (CurrentHP :type Integer) (CurrentEP :type Integer))
  (if IsDead
    (CallFunction|DeadNPC)
    (else
      (Default|ConfigLifebar (Variables|Default|GetBP_Char_Stats))
      (bind _asbp_widjet_npc_bar (Utilities|Casting|CastToBP_widjet_NPC_bar (UserInterface|GetUserWidgetObject (Variables|Default|GetWidget_NPC_healt))))
      (Variables|/Game/Blueprints/BP_HUD/BP_Widjet/BP_widjet_NPC_bar.BP_widjet_NPC_bar_C|SetNPC _asbp_widjet_npc_bar self))))