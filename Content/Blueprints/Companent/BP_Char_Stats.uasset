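; Character stats component that tracks HP, EP (shield), death and walk speed for its owner.
; BeginPlay and ConfigState load a data table row by name, with ConfigState also setting movement, refilling both pools and configuring the lifebar.
; Damage, heal and shield functions broadcast status updates, while Tick computes bar ratios.
; Damage bypasses EP, and a partial shield refill writes into CurrentHP instead of CurrentEP.
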(event EventBeginPlay
  (bind _returnvalue (Utilities|GetDataTableRow "/Game/Blueprints/Data/BP_DT_All_stats1.BP_DT_All_stats1" (Variables|Default|GetCurrenName))
    (:then
      (Variables|Default|SetMainStats _returnvalue)
      (Utilities|FlowControl|Sequence
        (:then_0
          (Variables|Default|SetCurrentHP (.MaxHP (Utilities|Struct|BreakBP_Main_Struct (Variables|Default|GetMainStats)))))
        (:then_1
          (Variables|Default|SetCurrentEP (.MaxEP (Utilities|Struct|BreakBP_Main_Struct (Variables|Default|GetMainStats)))))))))

(event EventTick
  (params (DeltaSeconds :type Float%20%28single-precision%29))
  (bind _mainstats (Variables|Default|GetMainStats))
  (bind (_maxhp _maxep) (Utilities|Struct|BreakBP_Main_Struct _mainstats))
  (Utilities|FlowControl|Sequence
    (:then_0
      (Variables|Default|SetLifebarFloat (/ (Math|Conversions|ToFloat(Integer) (Variables|Default|GetCurrentHP)) (Math|Conversions|ToFloat(Integer) _maxhp))))
    (:then_1
      (Variables|Default|SetEnergyFloat (/ (Math|Conversions|ToFloat(Integer) (Variables|Default|GetCurrentEP)) (Math|Conversions|ToFloat(Integer) _maxep))))))

(fn BPConfigState
  (bind _returnvalue (Utilities|GetDataTableRow "/Game/Blueprints/Data/BP_DT_All_stats1.BP_DT_All_stats1" (Variables|Default|GetCurrenName))
    (:then
      (Variables|Default|SetMainStats _returnvalue)
      (Utilities|FlowControl|Sequence
        (:then_0
          (Configuration|ConfigMove))
        (:then_1
          (CallFunction|HealUp true))
        (:then_2
          (CallFunction|ShieldUp true))
        (:then_3
          (Configuration|ConfigLifebar))))))

(fn ReceiveDamage
  (params (InDamage :type Float%20%28single-precision%29) (InType :type Byte) (InCauser :type Actor%20Object%20Reference))
  (if (not (Variables|Default|GetIsDead))
    (bind _output_get (Variables|Default|SetCurrentHP (- (Variables|Default|GetCurrentHP) (Math|Float|Truncate InDamage))))
    (if (> _output_get 0)
      (Variables|Default|SetIsDead false)
      (else
        (Variables|Default|SetCurrentHP 0)
        (Variables|Default|SetIsDead true)))
    (Default|CallOnStatusUpdate (Variables|Default|GetIsDead) true (Variables|Default|GetCurrentHP) (Variables|Default|GetCurrentEP))))

(fn BPHealUp
  (params (MaxRecover :type Boolean) (AddHP :type Integer))
  (if MaxRecover
    (Variables|Default|SetCurrentHP (Utilities|Struct|BreakBP_Main_Struct (Variables|Default|GetMainStats)))
    (else
      (Variables|Default|SetCurrentHP (Math|Integer|Min(Integer) (+ AddHP (Variables|Default|GetCurrentHP)) (Utilities|Struct|BreakBP_Main_Struct (Variables|Default|GetMainStats))))))
  (Default|CallOnStatusUpdate (Variables|Default|GetIsDead) false (Variables|Default|GetCurrentHP) (Variables|Default|GetCurrentEP)))

(fn BPShieldUp
  (params (MaxRecover :type Boolean) (Add_EP :type Integer))
  (if MaxRecover
    (Variables|Default|SetCurrentEP (Utilities|Struct|BreakBP_Main_Struct (Variables|Default|GetMainStats)))
    (else
      (Variables|Default|SetCurrentHP (Math|Integer|Min(Integer) (+ Add_EP (Variables|Default|GetCurrentEP)) (Utilities|Struct|BreakBP_Main_Struct (Variables|Default|GetMainStats))))))
  (Default|CallOnStatusUpdate (Variables|Default|GetIsDead) false (Variables|Default|GetCurrentHP) (Variables|Default|GetCurrentEP)))

(fn CheckHP
  (return (== (Variables|Default|GetCurrentHP) (Utilities|Struct|BreakBP_Main_Struct (Variables|Default|GetMainStats)))))

(fn CheckEP
  (return (== (Variables|Default|GetCurrentEP) (Utilities|Struct|BreakBP_Main_Struct (Variables|Default|GetMainStats)))))

(fn BPConfigMove
  (bind _mainstats (Variables|Default|GetMainStats))
  (bind _maxwolkspeed (Utilities|Struct|BreakBP_Main_Struct _mainstats))
  (if (Utilities|Enum|NotEqual(Enum) (Utilities|Struct|BreakBP_Main_Struct (Variables|Default|GetMainStats)) "NewEnumerator7")
    (bind _ascharacter (Utilities|Casting|CastToCharacter (Components|GetOwner)))
    (Variables|/Script/Engine.CharacterMovementComponent|SetMaxWalkSpeed (Variables|/Script/Engine.Character|GetCharacterMovement _ascharacter) _maxwolkspeed)
    (Variables|/Script/Engine.CharacterMovementComponent|SetMaxWalkSpeedCrouched (Variables|/Script/Engine.Character|GetCharacterMovement _ascharacter) (/ _maxwolkspeed 2.0))))

(fn BPConfigLifebar
  (bind _mainstats (Variables|Default|GetMainStats))
  (bind (_maxhp _maxep) (Utilities|Struct|BreakBP_Main_Struct _mainstats))
  (return (Utilities|String|Append (Utilities|GetDisplayName (Components|GetOwner)) " / " (Utilities|String|Append (Utilities|String|ToString(Integer) (Variables|Default|GetCurrentHP)) "/" (Utilities|String|ToString(Integer) _maxhp) "HP " (Utilities|String|ToString(Integer) (Variables|Default|GetCurrentEP)) "/" (Utilities|String|ToString(Integer) _maxep) "EP "))))